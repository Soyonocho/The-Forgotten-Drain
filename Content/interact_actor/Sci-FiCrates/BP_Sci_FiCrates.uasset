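; BP_Sci_FiCrates is a sci-fi crate that plays landing sounds on impact and supplies an item name with a visible prompt.
; Non-player mesh hits pick volume from velocity tiers and play sound through a Server-to-Multi event chain, gated by a DoOnce that resets at zero velocity.
; A hanging particle effect starts deactivated, then activates once when a delayed startup check or a hit finds the crate moving slowly.
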(event OnComponentHit(StaticMesh)
  (params (HitComponent :type Primitive%20Component%20Object%20Reference) (OtherActor :type Actor%20Object%20Reference) (OtherComp :type Primitive%20Component%20Object%20Reference) (NormalImpulse :type Vector :default "0, 0, 0") (Hit :type Hit%20Result%20Structure%20%28by%20ref%29))
  (bind _hitactor (Collision|BreakHitResult Hit))
  (bind _self self)
  (bind _self_2 self)
  (bind _returnvalue (Transformation|GetVelocity _self_2))
  (bind _returnvalue_2 (Transformation|GetVelocity _self))
  (bind _returnvalue_3 (Math|Vector|VectorLength _returnvalue))
  (bind _returnvalue_4 (Math|Vector|VectorLength _returnvalue_2))
  (if (not (== (Components|GetOwner) _hitactor))
    (if (not (Class|GameplayStatics|ObjectIsA _hitactor "/Game/FPMovement/Player/Blueprints/BP_Player.BP_Player_C"))
      (Utilities|FlowControl|Sequence
        (:then_0
          (Utilities|FlowControl|DoOnce false :!label _label
            (:Completed
              (if (and (>= _returnvalue_4 0.0) (< _returnvalue_4 5e+01))
                (Variables|Default|SetHitSoundVolume 0.2)
                (CallFunction|ServerPlaySound (Transformation|GetActorLocation) (Variables|Default|GetHitSoundVolume) :!label _label_2)
                (elif (and (>= _returnvalue_4 5e+01) (< _returnvalue_4 3e+02))
                  (Variables|Default|SetHitSoundVolume 0.5)
                  (goto _label_2)
                  (elif (>= _returnvalue_4 3e+02)
                    (Variables|Default|SetHitSoundVolume 1.0)
                    (goto _label_2)))))))
        (:then_1
          (if (== _returnvalue_3 0.0)
            (goto _label Reset)))
        (:then_2
          (if (<= _returnvalue_3 5e+01)
            (Utilities|FlowControl|DoOnce false
              (:Completed
                (Components|Activation|Activate (Variables|Default|GetHangingParticulate) false)))))))))

(event Custom|OnActorHit_Event
  (params (SelfActor :type Actor%20Object%20Reference) (OtherActor :type Actor%20Object%20Reference) (NormalImpulse :type Vector) (Hit :type Hit%20Result%20Structure%20%28by%20ref%29)))

(event Custom|ServerPlaySound
  (params (Location :type Vector) (VolumeMultiplier :type Float%20%28single-precision%29))
  (CallFunction|MultiPlaySound Location VolumeMultiplier))

(event Custom|MultiPlaySound
  (params (Location :type Vector) (VolumeMultiplier :type Float%20%28single-precision%29))
  (Audio|PlaySoundatLocation "/Game/interact_actor/Fruit/sound/land-81509.land-81509" Location "0, 0, 0" VolumeMultiplier 1.0 0.0 "/Game/interact_actor/Fruit/sound/fruti_land.fruti_land" 0 0 0))

(event Custom|LandedEvent
  (if (<= (Math|Vector|VectorLength (Transformation|GetVelocity self)) 5e+01)
    (Utilities|FlowControl|DoOnce false
      (:Completed
        (Components|Activation|Activate (Variables|Default|GetHangingParticulate) false)))))

(event Collision|EventActorBeginOverlap
  (params (OtherActor :type Actor%20Object%20Reference))
  (|CallParentFunction OtherActor) ; This node is disabled and will not be called.\nDrag off pins to build functionality.
)

(event EventTick
  (params (DeltaSeconds :type Float%20%28single-precision%29))
  (|CallParentFunction DeltaSeconds) ; This node is disabled and will not be called.\nDrag off pins to build functionality.
)

(event EventBeginPlay
  (Components|Activation|Deactivate (Variables|Default|GetHangingParticulate))
  (Utilities|FlowControl|Delay 0.1)
  (CallFunction|LandedEvent))

(fn ConstructionScript
  (|CallParentFunction))

(fn BPGetItemName
  (return (Variables|Default|GetItem%20Name) true))