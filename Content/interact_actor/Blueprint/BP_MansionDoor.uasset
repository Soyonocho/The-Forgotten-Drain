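; BP_MansionDoor is a double door with left and right leaves that swing open and closed independently.
; Each of two execute events checks whether its pivot sits at zero rotation, playing that leaf's timeline from the start if so and reversing it otherwise.
; The timelines lerp pivot yaw a quarter turn in opposite directions.
; Debug strings print on each call and timeline update.
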(event Custom|Open_MansionDoor_execute2
  (Development|PrintString "Dooropen")
  (if (Utilities|Operators|EqualEqual :B (Variables|/Script/Engine.SceneComponent|GetRelativeRotation (Variables|Default|GetRightDoorPivot)))
    (bind _newtrack_0 (Timeline|Timeline PlayFromStart)
      (:Update
        (Transformation|SetRelativeRotation (Variables|Default|GetRightDoorPivot) (Math|Rotator|MakeRotator 0.0 0.0 (Math|Float|Lerp 0.0 9e+01 _newtrack_0)) false false)
        (Development|PrintString "success")))
    (else
      (Timeline|Timeline Reverse))))

(event Custom|Open_MansionDoor_execute
  (Development|PrintString "Dooropen")
  (if (Utilities|Operators|EqualEqual :B (Variables|/Script/Engine.SceneComponent|GetRelativeRotation (Variables|Default|GetLeftDoorPivot)))
    (bind _newtrack_0 (Timeline|Door1 PlayFromStart)
      (:Update
        (Transformation|SetRelativeRotation (Variables|Default|GetLeftDoorPivot) (Math|Rotator|MakeRotator 0.0 0.0 (Math|Float|Lerp 0.0 -9e+01 _newtrack_0)) false false)
        (Development|PrintString "success")))
    (else
      (Timeline|Door1 Reverse))))

(fn ConstructionScript)