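; Enemy AI character that hunts a player and plays growls on a randomized repeating timer.
; Tick reads TargetActor from the AI controller's blackboard and calls Killed on that BP_Player at close range, with a DoOnce that rearms only once the target is far away.
; Sounds pass through server and multicast-named events to play at the enemy's location.
; Helpers set walk speed and restore walking movement on landing.
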(event Custom|PlaySound
  (params (WhichSound :type Integer))
  (CallFunction|PlaySoundServer WhichSound (Transformation|GetActorLocation)))

(event Custom|PlaySoundServer
  (params (WhichSound :type Integer) (Location :type Vector))
  (CallFunction|PlaySoundMulti WhichSound Location))

(event Custom|PlaySoundMulti
  (params (WhichSound :type Integer) (Location :type Vector))
  (Audio|PlaySoundatLocation (Utilities|Array|Get(acopy) (Variables|Default|GetSound) WhichSound) Location "0, 0, 0" 1.0 1.0 0.0 "/Game/AI/Sound/MonsterSound.MonsterSound" 0 0 0))

(event Custom|PlayDefaultSound
  (CallFunction|PlaySound 2)
  (Utilities|Time|SetTimerbyFunctionName 0 "PlayDefaultSound" (Math|Random|RandomFloatinRange 3.0 5.0))
  (Development|PrintString "growl"))

(event EventOnLanded
  (params (Hit :type Hit%20Result%20Structure%20%28by%20ref%29))
  (Pawn|Components|CharacterMovement|SetMovementMode (Variables|Character|GetCharacterMovement) "MOVE_Walking" 0))

(event Collision|EventActorBeginOverlap
  (params (OtherActor :type Actor%20Object%20Reference)))

(event EventTick
  (params (DeltaSeconds :type Float%20%28single-precision%29))
  (bind _returnvalue (Utilities|Name|MakeLiteralName "TargetActor"))
  (bind _returnvalue_2 (Transformation|GetActorLocation))
  (bind _self self)
  (bind _returnvalue_3 (AI|GetAIController _self))
  (bind _returnvalue_4 (AI|GetBlackboard _returnvalue_3))
  (bind _returnvalue_5 (AI|Components|Blackboard|GetValueasObject _returnvalue_4 _returnvalue))
  (bind _asbp_player (Utilities|Casting|CastToBP_Player _returnvalue_5))
  (bind _returnvalue_6 (Transformation|GetActorLocation _asbp_player))
  (bind _returnvalue_7 (Math|Vector|Distance(Vector) _returnvalue_6 _returnvalue_2))
  (if (Variables|Default|Getexite?)
    (if (Utilities|IsValid _returnvalue_3)
      (if (Utilities|IsValid _returnvalue_5)
        (if (<= _returnvalue_7 1e+02)
          (Utilities|FlowControl|DoOnce false :!label _label
            (:Completed
              (Default|Killed _asbp_player)
              (CallFunction|PlaySound 1)))
          (elif (>= _returnvalue_7 5e+02)
            (goto _label Reset)))))))

(event EventBeginPlay
  (Variables|Default|Setexite? true)
  (CallFunction|PlayDefaultSound))

(fn ConstructionScript)

(fn UpdateWalkSpeed
  (params (NewWalkSpeed :type Float%20%28double-precision%29))
  (Variables|/Script/Engine.CharacterMovementComponent|SetMaxWalkSpeed (Variables|Character|GetCharacterMovement) NewWalkSpeed))